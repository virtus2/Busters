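; Player character Blueprint, built on ALS overlay modes, that shows the held weapon for the current mode.
; Overlay changes link a mapped animation layer, falling back to the ALS default, and attach the M4 rifle or M9 pistol mesh to a socket or gun bone, or clear it.
; BeginPlay refreshes the weapon and activates the third-person camera over the ADS one.
; Left click plays a rifle shot animation on the ADS mesh.
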(event `self.ReceiveBeginPlay`
  (`self.RefreshOverlayObject`)
  (`ActorComponent.SetActive` (`self.ADSCamera`) false false)
  (`ActorComponent.SetActive` (`self.ThirdPersonCamera`) true false))

(event `self.OnOverlayModeChanged`
  (params (PreviousModeTag :type "GameplayTag Structure (by ref)"))
  (`self.RefreshOverlayLinkedAnimationLayer`)
  (`self.RefreshOverlayObject`))

(event `Key|LeftMouseButton`
  (params (Key :type "Key Structure"))
  (:`Pressed`
    (`SkeletalMeshComponent.PlayAnimation` (`self.ADSSkeletalMesh`) "/Game/FPS_Assault_Pack/Animations/Rifle/A_Rifle_Shoot01.A_Rifle_Shoot01" false)))

(fn `AttachOverlayObject`
  (params (NewStaticMesh :type "StaticMesh Object Reference") (NewSkeletalMesh :type "SkeletalMesh Object Reference") (NewAnimationClass :type "AnimInstance Class Reference") (SocketName :type Name) (bUseLeftGunBone :type Boolean))
  (locals (ResultSocketName :type Name))
  (set `local.ResultSocketName` (select `bool` (`self.bUseGunBoneForOverlayObjects`) :`false` (`local.SocketName`) :`true` (select `bool` (`local.bUseLeftGunBone`) :`false` (`AlsConstants.HandRightGunVirtualBone`) :`true` (`AlsConstants.HandLeftGunVirtualBone`))))
  (`|ExecutionSequence`
    (:`then_0`
      (`StaticMeshComponent.SetStaticMesh` (`self.OverlayStaticMesh`) (`local.NewStaticMesh`))
      (`SceneComponent.K2_AttachToComponent` (`self.OverlayStaticMesh`) (`self.Mesh`) (`local.ResultSocketName`) "SnapToTarget" "SnapToTarget" "SnapToTarget" true))
    (:`then_1`
      (`SkinnedMeshComponent.SetSkinnedAssetAndUpdate` (`self.OverlaySkeletalMesh`) (`local.NewSkeletalMesh`) true)
      (`SkeletalMeshComponent.SetAnimInstanceClass` (`self.OverlaySkeletalMesh`) (`local.NewAnimationClass`))
      (`SceneComponent.K2_AttachToComponent` (`self.OverlaySkeletalMesh`) (`self.Mesh`) (`local.ResultSocketName`) "SnapToTarget" "SnapToTarget" "SnapToTarget" true))))

(fn `ClearOverlayObject`
  (`StaticMeshComponent.SetStaticMesh` (`self.OverlayStaticMesh`) null)
  (`SkinnedMeshComponent.SetSkinnedAssetAndUpdate` (`self.OverlaySkeletalMesh`) null true)
  (`SkeletalMeshComponent.SetAnimInstanceClass` (`self.OverlaySkeletalMesh`) null))

(fn `NewFunction_0`
  (returns (ThirdPersonCamera :type "CameraComponent Object Reference"))
  (return (`self.ThirdPersonCamera`)))

(fn `RefreshOverlayLinkedAnimationLayer`
  (locals (OverlayAnimationInstanceClass :type "AnimInstance Class Reference"))
  (bind _mesh (`self.Mesh`))
  (set `local.OverlayAnimationInstanceClass` (`BlueprintMapLibrary.Map_Find` (`self.OverlayAnimationInstanceClasses`) (`self.OverlayMode`)))
  (bind _overlayanimationinstanceclass (`local.OverlayAnimationInstanceClass`)
    (:`then`
      (`SkeletalMeshComponent.LinkAnimClassLayers` _mesh _overlayanimationinstanceclass))
    (:`else`
      (`SkeletalMeshComponent.LinkAnimClassLayers` _mesh "/ALS/ALS/Character/AnimationInstances/Overlays/AB_Als_Default.AB_Als_Default_C"))))

(fn `RefreshOverlayObject`
  (`|SwitchGameplayTag` (`self.OverlayMode`)
    (:`Default`
      (`self.ClearOverlayObject`))
    (:`Als.OverlayMode.M4`
      (`self.AttachOverlayObject` null "/Game/FPS_Assault_Pack/Meshes/Rifle/SK_Rifle.SK_Rifle" null "M4"))
    (:`Als.OverlayMode.PistolTwoHanded`
      (`self.AttachOverlayObject` null "/ALS/ALS/OverlayObjects/M9/SKM_M9.SKM_M9" null "M9"))))

(fn `UserConstructionScript`)